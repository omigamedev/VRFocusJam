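; BP_Pawn is a motion-controller pawn that lets the right hand drag interactive actors.
; BoxR overlaps remember the latest BPI_Interactive actor, which end overlap never clears.
; The right trigger starts and ends a drag on that actor through Begin and End messages, printing a debug string.
; While dragging, Tick sends it the box's world location and total offset from the drag start.
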(event `self.ReceiveTick`
  (params (DeltaSeconds :type "Float (single-precision)"))
  (bind _returnvalue (`SceneComponent.K2_GetComponentLocation` (`self.BoxR`)))
  (if (and (`KismetSystemLibrary.IsValid` (`self.CurrentOverlapR`)) (`self.bDraggingR`))
    (message `/Game/SuperHands/Blueprints/BPI_Interactive.DragUpdate` (`self.CurrentOverlapR`) _returnvalue (- _returnvalue (`self.DragStartR`)))))

(event `self.BoxR.OnComponentBeginOverlap`
  (params (OverlappedComponent :type "PrimitiveComponent Object Reference") (OtherActor :type "Actor Object Reference") (OtherComp :type "PrimitiveComponent Object Reference") (OtherBodyIndex :type Integer) (bFromSweep :type Boolean) (SweepResult :type "HitResult Structure (by ref)"))
  (if (`KismetSystemLibrary.DoesImplementInterface` OtherActor "/Game/SuperHands/Blueprints/BPI_Interactive.BPI_Interactive_C")
    (set `self.CurrentOverlapR` OtherActor)))

(event `self.BoxR.OnComponentEndOverlap`
  (params (OverlappedComponent :type "PrimitiveComponent Object Reference") (OtherActor :type "Actor Object Reference") (OtherComp :type "PrimitiveComponent Object Reference") (OtherBodyIndex :type Integer))
  (if (and (`KismetSystemLibrary.IsValid` (`self.CurrentOverlapR`)) (`self.bDraggingR`))
    _))

(event `Key|MotionController_Right_Trigger`
  (params (Key :type "Key Structure" :default "AnyKey"))
  (:`Pressed`
    (if (`KismetSystemLibrary.IsValid` (`self.CurrentOverlapR`))
      (set `self.bDraggingR` true)
      (bind _output_get (set `self.DragStartR` (`SceneComponent.K2_GetComponentLocation` (`self.BoxR`))))
      (message `/Game/SuperHands/Blueprints/BPI_Interactive.DragBegin` (`self.CurrentOverlapR`) _output_get)
      (`KismetSystemLibrary.PrintString` "Hello" :!label _label)))
  (:`Released`
    (set `self.bDraggingR` false)
    (if (`KismetSystemLibrary.IsValid` (`self.CurrentOverlapR`))
      (message `/Game/SuperHands/Blueprints/BPI_Interactive.DragEnd` (`self.CurrentOverlapR`))
      (goto _label))))

(fn `UserConstructionScript`)