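; Dumbion pawn that walks forward constantly and is steered by dragging.
; Each tick, MoveForward sets the physics capsule's horizontal velocity from the skeletal mesh's forward vector and Speed, keeping vertical velocity intact.
; DragUpdate turns the mesh to face the drag delta, which redirects the movement.
; Disconnected nodes hold an unused steering approach based on hand overlap with a box and an arrow indicator.
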(event `/Game/SuperHands/Blueprints/BPI_Interactive.DragBegin`
  (params (Location :type "Vector Structure")))

(event `/Game/SuperHands/Blueprints/BPI_Interactive.DragUpdate`
  (params (Location :type "Vector Structure") (Delta :type "Vector Structure"))
  (`SceneComponent.K2_SetWorldRotation` (`self.SkeletalMesh`) (`KismetMathLibrary.Conv_VectorToRotator` Delta) false false))

(event `/Game/SuperHands/Blueprints/BPI_Interactive.DragEnd`)

(event `self.ReceiveTick`
  (params (DeltaSeconds :type "Float (single-precision)"))
  (`self.MoveForward`))

(event `Key|MotionController_Left_Trigger` :consume false
  (params (Key :type "Key Structure" :default "AnyKey")))

(event `Key|MotionController_Right_Trigger` :consume false
  (params (Key :type "Key Structure" :default "AnyKey")))

(fn `MoveForward`
  (bind _capsule (`self.Capsule`))
  (bind (_returnvalue_x _returnvalue_y) (`KismetMathLibrary.BreakVector` (* (`SceneComponent.GetForwardVector` (`self.SkeletalMesh`)) (`self.Speed`))))
  (bind _returnvalue (`PrimitiveComponent.GetPhysicsLinearVelocity` _capsule "None"))
  (`PrimitiveComponent.SetPhysicsLinearVelocity` _capsule (`KismetMathLibrary.MakeVector` _returnvalue_x _returnvalue_y (.z _returnvalue)) false "None"))

(fn `UserConstructionScript`)